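; BP_Goblin is a goblin enemy character that varies its look and handles its own death.
; The construction script creates a dynamic material instance on the mesh and randomly picks one of two goblin textures.
; KillPawn disables capsule collision, plays the lose montage, then destroys the actor whether the montage completes or is interrupted.
; On unpossess, any playing montage is stopped to avoid a PIE crash.
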(event Custom|KillPawn
  ;[1 1 1] Play dead montage and destroy
  (Collision|SetCollisionEnabled (Variables|Collision|GetCapsuleComponent) "NoCollision")
  (Animation|Montage|PlayMontage (Variables|Character|GetMesh) "/Game/UndeadPack/EnemyGoblin/Animations/Anim_Lose_Montage.Anim_Lose_Montage"
    (:OnCompleted
      _)
    (:OnInterrupted
      _))
  (Actor|DestroyActor))

(event EventUnpossessed
  (params (OldController :type Controller%20Object%20Reference))
  (bind _returnvalue (Animation|GetCurrentMontage :!class /Script/Engine.Character))
  ;[1 1 1] Stop PIE crash if we keep montage plaing
  (Utilities|IsValid _returnvalue
    (:Is%20Valid
      (Animation|StopAnimMontage _returnvalue))))

(fn ConstructionScript
  (CallFunction|RandomizeMaterial))

(fn RandomizeMaterial
  (bind _returnvalue (Rendering|Material|CreateDynamicMaterialInstance (Variables|Character|GetMesh) 0 "/Game/UndeadPack/EnemyGoblin/Materials/M_EnemyGoblin.M_EnemyGoblin" "None" :!class /Script/Engine.PrimitiveComponent))
  (Rendering|Material|SetTextureParameterValue _returnvalue "Texture" (Utilities|Select :Index (Math|Random|RandomIntegerinRange 0 1) :Option%200 "/Game/UndeadPack/EnemyGoblin/Textures/T_EG_02_D.T_EG_02_D" :Option%201 "/Game/UndeadPack/EnemyGoblin/Textures/T_EG_01_D.T_EG_01_D")))
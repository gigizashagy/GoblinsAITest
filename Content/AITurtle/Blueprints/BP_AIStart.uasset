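; BP_AIStart is an interactable spawn point that summons an AI character and sends it toward a destination.
; On Interact it spawns the configured class at its own transform and plays a Niagara summon effect.
; It passes the start location, a destination defined in the actor's local space, and a sub behavior tree to the spawned character's BP_AIController.
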(event EventInteract
  (params (Instigator :type Actor%20Object%20Reference))
  ;[1 1 1] Interaction
  (CallFunction|SpawnAI)
  (CallFunction|SpawnEffect))

(fn ConstructionScript)

(fn SpawnAI
  (bind _returnvalue (Game|SpawnActorfromClass (Variables|Default|GetAICLass) (Transformation|GetActorTransform) "AdjustIfPossibleButAlwaysSpawn" 0 0))
  (bind _ascharacter (Utilities|Casting|CastToCharacter _returnvalue))
  (bind _asbp_aicontroller (Utilities|Casting|CastToBP_AIController (Pawn|GetController _ascharacter)))
  (Default|SetStartandDestination _asbp_aicontroller (Math|Transform|TransformLocation (Transformation|GetActorTransform) (Variables|Default|GetDestinationLocation)) (Transformation|GetActorLocation))
  (Default|SetSubBehavior _asbp_aicontroller (Variables|Default|GetSubBehaviorTree)))

(fn SpawnEffect
  (Niagara|SpawnSystematLocation "/Game/AITurtle/Effects/FX_Ability/Summon/P_Summon_Parent_Startup_Converted.P_Summon_Parent_Startup_Converted" (Transformation|GetActorLocation)))